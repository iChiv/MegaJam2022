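; BP_MagGunUltra is a magnet gun that pulls a BP_MetalBall toward its Mag component while Q is held.
; Q sets a pressed flag, and Tick then looks up a single ball by class and applies a mass-independent, distance-independent MagForce along the normalized direction to Mag.
; The construction script applies configurable transforms to GunBody and Mag, and debug prints trace input and the pull vector.
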(event `self.ReceiveBeginPlay`
  (`self.EnableInput` (`GameplayStatics.GetPlayerController` 0)))

(event `self.ReceiveTick`
  (params (DeltaSeconds :type "Float (single-precision)"))
  (if (`self.IsPressed`)
    (bind _returnvalue (`GameplayStatics.GetActorOfClass` "/Game/BPs/BP_MetalBall.BP_MetalBall_C" :!label _label))
    (bind _output_get (set `self.SubVec` (- (`SceneComponent.K2_GetComponentLocation` (`self.Mag`)) (`self.K2_GetActorLocation` _returnvalue))))
    (bind _returnvalue_2 (`KismetStringLibrary.Conv_VectorToString` _output_get))
    (`KismetSystemLibrary.PrintString` _returnvalue_2)
    (`PrimitiveComponent.AddForce` (`/Game/BPs/BP_MetalBall.Ball` _returnvalue) (* _output_get (* (`self.MagForce`) (/ 1.0 (`KismetMathLibrary.VSize` _output_get)))) "None" true)
    (`KismetSystemLibrary.PrintString` _returnvalue_2)))

(event `Key|Q`
  (params (Key :type "Key Structure"))
  (:`Pressed`
    (`KismetSystemLibrary.PrintString` "EEEEEEEEEEEEEEEE")
    (set `self.IsPressed` true)
    (goto _label))
  (:`Released`
    (`KismetSystemLibrary.PrintString` "RRRRRRRRRRRRRRRRR")
    (set `self.IsPressed` false)))

(fn `UserConstructionScript`
  (`SceneComponent.K2_SetRelativeTransform` (`self.GunBody`) (`self.GunSize`) false false)
  (`SceneComponent.K2_SetRelativeTransform` (`self.Mag`) (`self.MagCenter`) false false))