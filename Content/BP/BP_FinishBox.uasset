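; BP_FinishBox is a level goal trigger that reacts when a BP_MetalPlus overlaps its CheckBox.
; It shows the Win component, plays LevelSuccess, then hides itself and advances a wrapping level counter.
; It then tells BP_LevelMeshes to change mesh, repositions the metal and calls SwitchBox00 on BP_MachinBox, reappearing after a delay.
; Ending the overlap hides Win again.
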(event `self.CheckBox.OnComponentBeginOverlap`
  (params (OverlappedComponent :type "PrimitiveComponent Object Reference") (OtherActor :type "Actor Object Reference") (OtherComp :type "PrimitiveComponent Object Reference") (OtherBodyIndex :type Integer) (bFromSweep :type Boolean) (SweepResult :type "HitResult Structure (by ref)"))
  (cast `/Game/BP/BP_MetalPlus` OtherActor)
  (`SceneComponent.SetHiddenInGame` (`self.Win`) false false)
  (`AudioComponent.Play` (`self.Level_Success`) 0.0)
  (`KismetSystemLibrary.Delay` 1.0)
  (`self.SetActorHiddenInGame` true)
  ;[1 1 1] Judge Level Number
  (bind _result (`/Engine/EditorBlueprintResources/StandardMacros.IncrementInt` (`self.FinishBoxNum`))
    (:`  `
      (if (not (< _result 3))
        (set `self.FinishBoxNum` 0))
      (bind _outactors (`GameplayStatics.GetAllActorsOfClass` "/Game/BP/BP_LevelMeshes.BP_LevelMeshes_C"))
      (`/Game/BP/BP_LevelMeshes.ChangeStaticMesh` (`|GetArrayItem` _outactors))
      (bind _asbp_metal_plus (cast `/Game/BP/BP_MetalPlus` OtherActor))
      (`/Game/BP/BP_MetalPlus.RepositionMetalPlus` _asbp_metal_plus)
      (bind _returnvalue (`GameplayStatics.GetActorOfClass` "/Game/BP/BP_MachinBox.BP_MachinBox_C"))
      (`/Game/BP/BP_MachinBox.SwitchBox00` _returnvalue)
      (`KismetSystemLibrary.Delay` 5.0)
      (`self.SetActorHiddenInGame` false))))

(event `self.CheckBox.OnComponentEndOverlap`
  (params (OverlappedComponent :type "PrimitiveComponent Object Reference") (OtherActor :type "Actor Object Reference") (OtherComp :type "PrimitiveComponent Object Reference") (OtherBodyIndex :type Integer))
  (cast `/Game/BP/BP_MetalPlus` OtherActor)
  (`SceneComponent.SetHiddenInGame` (`self.Win`) true false))

(fn `UserConstructionScript`)