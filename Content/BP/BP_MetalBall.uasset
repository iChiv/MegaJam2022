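; BP_MetalBall is a physics ball that gets pulled toward another actor while E or the right trigger is held, like a magnet.
; BeginPlay enables player input, and pressing starts a timeline whose play rate comes from AttractTime; releasing stops it.
; Each timeline update finds the target by class and applies acceleration along the unnormalized offset, so the pull grows with distance.
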(event `self.ReceiveBeginPlay`
  (`self.EnableInput` (`GameplayStatics.GetPlayerController` 0)))

(event `Key|E`
  (params (Key :type "Key Structure"))
  (:`Pressed`
    (`KismetSystemLibrary.PrintString` "EEEEEEEEEEEEEEEE" :!label _label)
    (`TimelineComponent.SetPlayRate` (`self.TL_Ball`) (/ 1.0 (`self.AttractTime`)))
    (`Timeline|TL_Ball` :!via `PlayFromStart` :!label _label_2
      (:`Update`
        (bind _returnvalue (`GameplayStatics.GetActorOfClass` null))
        (bind _output_get (set `self.SubtractedVector` (- (`self.K2_GetActorLocation` _returnvalue) (`SceneComponent.K2_GetComponentLocation` (`self.Ball`)))))
        (`PrimitiveComponent.AddForce` (`self.Ball`) (* _output_get (50.0 50.0 50.0)) "None" true)
        (`KismetSystemLibrary.PrintString` "Working!"))))
  (:`Released`
    (`KismetSystemLibrary.PrintString` "RRRRRRRRRRRRRRRRR" :!label _label_3)
    (goto _label_2 :!via `Stop`)))

(event `InputAction|TriggerRight`
  (params (Key :type "Key Structure"))
  (:`Pressed`
    (goto _label))
  (:`Released`
    (goto _label_3)))

(fn `UserConstructionScript`)