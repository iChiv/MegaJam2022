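; BP_MagGun is a magnet gun that pulls a BP_MetalBall toward its Mag component when the trigger is pressed.
; Each press finds one ball by class and applies a single mass-independent AddForce along the normalized direction, scaled by MagForce.
; Trigger events also set IsPressed, which nothing here reads, and print debug strings.
; The construction script sets GunBody and Mag relative transforms from variables.
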(event `/Game/VRTemplate/Blueprints/VRInteractionBPI.TriggerPressed`
  (`KismetSystemLibrary.PrintString` "EEEEEEEEEEEEEEEE")
  (set `self.IsPressed` true)
  (bind _returnvalue (`GameplayStatics.GetActorOfClass` "/Game/BP/BP_MetalBall.BP_MetalBall_C"))
  (bind _output_get (set `self.SubVec` (- (`SceneComponent.K2_GetComponentLocation` (`self.Mag`)) (`self.K2_GetActorLocation` _returnvalue))))
  (bind _returnvalue_2 (`KismetStringLibrary.Conv_VectorToString` _output_get))
  (`KismetSystemLibrary.PrintString` _returnvalue_2)
  (`PrimitiveComponent.AddForce` (`/Game/BP/BP_MetalBall.Ball` _returnvalue) (* _output_get (* (`self.MagForce`) (/ 1.0 (`KismetMathLibrary.VSize` _output_get)))) "None" true)
  (`KismetSystemLibrary.PrintString` _returnvalue_2))

(event `/Game/VRTemplate/Blueprints/VRInteractionBPI.TriggerReleased`
  (`KismetSystemLibrary.PrintString` "RRRRRRRRRRRRRRRRR")
  (set `self.IsPressed` false))

(fn `UserConstructionScript`
  (`SceneComponent.K2_SetRelativeTransform` (`self.GunBody`) (`self.GunSize`) false false)
  (`SceneComponent.K2_SetRelativeTransform` (`self.Mag`) (`self.MagCenter`) false false))