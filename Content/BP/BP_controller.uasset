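; BP_controller is a grabbable controller that pushes a referenced Bot by remote.
; Pressing the right trigger applies one force to the Bot's body along the vector from the controller's Antenna to the Bot, scaled by Strength.
; The vector is not normalized, so the push grows with distance.
; GrabComponent events toggle actor tick, but the graph has no Tick logic and the trigger handler does not check grab state.
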(event `self.GrabComponent.OnGrabbed`
  (`self.SetActorTickEnabled` true))

(event `self.GrabComponent.OnDropped`
  (`self.SetActorTickEnabled` false))

(event `InputAction|TriggerRight`
  (params (Key :type "Key Structure"))
  (:`Pressed`
    (`PrimitiveComponent.AddForce` (`/Game/BP/BP_robots.botBody` (`self.Bot`)) (* (- (`self.K2_GetActorLocation` (`self.Bot`)) (`SceneComponent.K2_GetComponentLocation` (`self.antenna`))) (`self.Strength`)) "None" false)))

(fn `UserConstructionScript`)