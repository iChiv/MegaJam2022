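; Battery-powered VR magnetic wrench that pulls the BP_MetalPlus actor toward its BallPosition while the trigger is held.
; Each powered Tick applies constant-magnitude acceleration to the metal's sphere, drains Battery and plays distance-scaled haptics on the holding hand.
; Trigger events toggle the pull, with magnetic effects shown on wrench and target; dropping also stops the pull.
; SetBattery resets charge to a base plus a bonus from BP_FinishBox's FinishBoxNum.
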(event `self.ReceiveTick`
  (params (DeltaSeconds :type "Float (single-precision)"))
  (if (> (`self.Battery`) 0.0)
    (if (`self.IsPressed`)
      (bind _returnvalue (`GameplayStatics.GetActorOfClass` "/Game/BP/BP_MetalPlus.BP_MetalPlus_C"))
      (bind _returnvalue_2 (- (`SceneComponent.K2_GetComponentLocation` (`self.BallPosition`)) (`self.K2_GetActorLocation` _returnvalue)))
      (set `self.ForceDir` _returnvalue_2)
      (`PrimitiveComponent.AddForce` (`/Game/BP/BP_MetalPlus.Sphere` _returnvalue) (* (`self.ForceDir`) (* (`self.MagForce`) (/ 1.0 (`KismetMathLibrary.VSize` _returnvalue_2)))) "None" true)
      (`self.PlayHapticEffect` (/ (`self.GetDistanceTo` _returnvalue) 100.0))
      (bind _output_get (set `self.Battery` (- (`self.Battery`) (`self.BatteryReduce`))))
      (`KismetSystemLibrary.PrintString` (`KismetStringLibrary.Conv_DoubleToString` _output_get))
      (`SceneComponent.SetHiddenInGame` (`self.P_MagneticVFX`) false false)
      (bind _returnvalue_3 (`GameplayStatics.GetActorOfClass` "/Game/BP/BP_MetalPlus.BP_MetalPlus_C"))
      (`SceneComponent.SetHiddenInGame` (`SceneComponent.GetChildComponent` (`/Game/BP/BP_MetalPlus.Sphere` _returnvalue_3) 2) false false))))

(event `/Game/VRTemplate/Blueprints/VRInteractionBPI.TriggerPressed`
  (set `self.IsPressed` true)
  (`AudioComponent.Play` (`self.WrenchActivated`) 0.0))

(event `/Game/VRTemplate/Blueprints/VRInteractionBPI.TriggerReleased`
  (set `self.IsPressed` false)
  (`SceneComponent.SetHiddenInGame` (`self.P_MagneticVFX`) true false)
  (bind _returnvalue (`GameplayStatics.GetActorOfClass` "/Game/BP/BP_MetalPlus.BP_MetalPlus_C"))
  (`SceneComponent.SetHiddenInGame` (`SceneComponent.GetChildComponent` (`/Game/BP/BP_MetalPlus.Sphere` _returnvalue) 2) true false))

(event `self.GrabComponentSnap.OnDropped`
  (set `self.IsPressed` false))

(event `SetBattery`
  (set `self.Battery` 50.0)
  (bind _returnvalue (`GameplayStatics.GetActorOfClass` "/Game/BP/BP_FinishBox.BP_FinishBox_C"))
  (set `self.Battery` (+ (* (`/Game/BP/BP_FinishBox.FinishBoxNum` _returnvalue) 25) (`self.Battery`))))

(fn `PlayHapticEffect`
  (params (HapticIntensity :type "Float (single-precision)"))
  ;[0.03434 0.03434 0.03434] Play Haptic Effect
  (`PlayerController.PlayHapticEffect` (`GameplayStatics.GetPlayerController` 0) (`self.PistolFireHapticEffect`) (select `bool` (== (`MotionControllerComponent.MotionSource` (`/Game/VRTemplate/Blueprints/GrabComponent.MotionControllerRef` (`self.GrabComponentSnap`))) "Left") :`false` "Right" :`true` "Left" :!type "EControllerHand Enum") HapticIntensity false))

(fn `UserConstructionScript`)