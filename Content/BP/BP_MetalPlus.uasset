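; BP_MetalPlus is an actor with a Sphere component that can be sent back to its starting position.
; BeginPlay stores the Sphere's world location, and RepositionMetalPlus restores it after a short delay.
; Tick toggles BallRolling by comparing LastLocation to the current location, but LastLocation is overwritten just beforehand, so it calls Play every frame and the Stop branch is effectively unreachable.
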(event `self.ReceiveTick`
  (params (DeltaSeconds :type "Float (single-precision)"))
  (set `self.lastLocation` (`SceneComponent.K2_GetComponentLocation` (`self.Sphere`)))
  (if (== (`self.lastLocation`) (`SceneComponent.K2_GetComponentLocation` (`self.Sphere`)))
    (`AudioComponent.Play` (`self.BallRolling`) 0.0)
    (else
      (`AudioComponent.Stop` (`self.BallRolling`)))))

(event `self.ReceiveBeginPlay`
  (set `self.SpawnLocation` (`SceneComponent.K2_GetComponentLocation` (`self.Sphere`))))

(event `RepositionMetalPlus`
  (`KismetSystemLibrary.Delay` 1.5)
  (`SceneComponent.K2_SetWorldLocation` (`self.Sphere`) (`self.SpawnLocation`) false false))

(fn `UserConstructionScript`)