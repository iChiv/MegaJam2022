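; BP_MagGunPlusBackup is a magnet gun that pulls a BP_MetalPlus ball to itself while the trigger is held.
; Trigger press finds a BP_MetalPlus actor by class, with no trace or range check, and grabs its Sphere with a PhysicsHandle.
; Tick keeps the handle target at the BallPosition component's world location, and trigger release drops the grabbed component.
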(event `self.ReceiveTick`
  (params (DeltaSeconds :type "Float (single-precision)"))
  (`PhysicsHandleComponent.SetTargetLocation` (`self.PhysicsHandle`) (`SceneComponent.K2_GetComponentLocation` (`self.BallPosition`))))

(event `/Game/VRTemplate/Blueprints/VRInteractionBPI.TriggerPressed`
  (bind _returnvalue (`GameplayStatics.GetActorOfClass` "/Game/BP/BP_MetalPlus.BP_MetalPlus_C"))
  (bind _sphere (`/Game/BP/BP_MetalPlus.Sphere` _returnvalue))
  (`PhysicsHandleComponent.GrabComponentAtLocation` (`self.PhysicsHandle`) _sphere "None" (`SceneComponent.K2_GetComponentLocation` _sphere)))

(event `/Game/VRTemplate/Blueprints/VRInteractionBPI.TriggerReleased`
  (`PhysicsHandleComponent.ReleaseComponent` (`self.PhysicsHandle`)))

(fn `UserConstructionScript`)