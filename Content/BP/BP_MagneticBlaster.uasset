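; BP_MagneticBlaster is a grabbable VR tool that magnetically pulls a BP_MetalPlus actor while the trigger is held.
; Pressing the trigger plays WrenchActivated, while releasing it or dropping the tool stops the pull.
; Each tick, it finds one BP_MetalPlus and accelerates its Sphere toward BallPosition at constant MagForce, regardless of distance.
; It also pulses haptics on the holding hand, scaled up with distance to the target.
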(event `self.ReceiveTick`
  (params (DeltaSeconds :type "Float (single-precision)"))
  (if (`self.IsPressed`)
    (bind _returnvalue (`GameplayStatics.GetActorOfClass` "/Game/BP/BP_MetalPlus.BP_MetalPlus_C"))
    (bind _returnvalue_2 (- (`SceneComponent.K2_GetComponentLocation` (`self.BallPosition`)) (`self.K2_GetActorLocation` _returnvalue)))
    (set `self.ForceDir` _returnvalue_2)
    (`PrimitiveComponent.AddForce` (`/Game/BP/BP_MetalPlus.Sphere` _returnvalue) (* (`self.ForceDir`) (* (`self.MagForce`) (/ 1.0 (`KismetMathLibrary.VSize` _returnvalue_2)))) "None" true)
    (`self.PlayHapticEffect` (/ (`self.GetDistanceTo` _returnvalue) 100.0))))

(event `/Game/VRTemplate/Blueprints/VRInteractionBPI.TriggerPressed`
  (set `self.IsPressed` true)
  (`AudioComponent.Play` (`self.WrenchActivated`) 0.0))

(event `/Game/VRTemplate/Blueprints/VRInteractionBPI.TriggerReleased`
  (set `self.IsPressed` false))

(event `self.GrabComponentSnap.OnDropped`
  (set `self.IsPressed` false))

(fn `PlayHapticEffect`
  (params (HapticIntensity :type "Float (single-precision)"))
  ;[0.03434 0.03434 0.03434] Play Haptic Effect
  (`PlayerController.PlayHapticEffect` (`GameplayStatics.GetPlayerController` 0) (`self.PistolFireHapticEffect`) (select `bool` (== (`MotionControllerComponent.MotionSource` (`/Game/VRTemplate/Blueprints/GrabComponent.MotionControllerRef` (`self.GrabComponentSnap`))) "Left") :`false` "Right" :`true` "Left" :!type "EControllerHand Enum") HapticIntensity false))

(fn `UserConstructionScript`)