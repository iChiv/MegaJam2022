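; BP_MachinBox animates the Box00 component through a machine-like cycle when its SwitchBox00 event fires.
; The box eases along its relative X axis, pauses briefly, snaps to a fixed lower position, then eases upward, which suggests a replacement box appearing.
; The sequence chains latent MoveComponentTo and Delay nodes in the event graph, with no Timeline or Tick and an empty construction script.
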(event `SwitchBox00`
  (bind _box00 (`self.Box00`))
  (bind _box00_2 (`self.Box00`))
  (bind (_relativelocation_x _relativelocation_y _relativelocation_z) (`KismetMathLibrary.BreakVector` (`SceneComponent.RelativeLocation` _box00_2)))
  (bind (_relativelocation_x_2 _relativelocation_y_2 _relativelocation_z_2) (`KismetMathLibrary.BreakVector` (`SceneComponent.RelativeLocation` _box00)))
  (`KismetSystemLibrary.MoveComponentTo` _box00_2 (`KismetMathLibrary.MakeVector` (+ _relativelocation_x 100.0) _relativelocation_y _relativelocation_z) (`SceneComponent.RelativeRotation` _box00_2) false true 2.0)
  (`KismetSystemLibrary.Delay` 0.5)
  (`SceneComponent.K2_SetRelativeLocation` (`self.Box00`) (65.0 60.0 -40.0) false false)
  (`KismetSystemLibrary.MoveComponentTo` _box00 (`KismetMathLibrary.MakeVector` _relativelocation_x_2 _relativelocation_y_2 (+ _relativelocation_z_2 47.0)) (`SceneComponent.RelativeRotation` _box00) false true 2.0))

(fn `UserConstructionScript`)